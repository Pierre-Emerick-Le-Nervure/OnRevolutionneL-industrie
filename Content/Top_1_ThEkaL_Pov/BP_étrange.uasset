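; BP_étrange is an actor that gradually scatters Bp_Bobcible actors around itself once play begins.
; A delayed loop repeatedly picks a random direction and distance, runs a line trace, and spawns a target facing back toward this actor.
; Spawns use the trace's end point rather than the impact, so obstacles do not affect placement.
; The capsule overlap compares the other actor to the player controller but triggers nothing.
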(event `self.ReceiveBeginPlay`
  (bind _returnvalue (`self.K2_GetActorLocation`))
  (`/Game/Top_1_ThEkaL_Pov/NewMacroLibrary.For loop with delay` 0 1000 0.1
    (:`NewParam5`
      (bind _outhit (`KismetSystemLibrary.LineTraceSingle` (+ _returnvalue (0.0 0.0 0.0)) (+ (* (`KismetMathLibrary.RandomUnitVector`) (`KismetMathLibrary.RandomFloatInRange` 1500.0 2500.0)) _returnvalue) "TraceTypeQuery1"))
      (bind (_bblockinghit _binitialoverlap _time _distance _location _impactpoint _normal _impactnormal _physmat _hitactor _hitcomponent _hitbonename _bonename _hititem _elementindex _faceindex _tracestart _traceend) (`GameplayStatics.BreakHitResult` _outhit))
      (`|SpawnActorFromClass` "/Game/Top_1_ThEkaL_Pov/Bp_Bobcible.Bp_Bobcible_C" (`KismetMathLibrary.MakeTransform` _traceend (`KismetMathLibrary.FindLookAtRotation` _traceend _returnvalue)) "Undefined" "MultiplyWithRoot" null null))))

(event `self.Capsule.OnComponentBeginOverlap`
  (params (OverlappedComponent :type "PrimitiveComponent Object Reference") (OtherActor :type "Actor Object Reference") (OtherComp :type "PrimitiveComponent Object Reference") (OtherBodyIndex :type Integer) (bFromSweep :type Boolean) (SweepResult :type "HitResult Structure (by ref)"))
  (if (== OtherActor (`GameplayStatics.GetPlayerController` 0))
    _))

(fn `UserConstructionScript`)